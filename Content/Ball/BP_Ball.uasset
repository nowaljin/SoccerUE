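; BP_Ball is a ball that reacts to the player's foot by replacing itself with a BP_Ball_Hi actor.
; When the Sphere overlaps a third-person character's FootCapsule, a DoOnce calls BallHiSpawnFunc, hides the ball, disables collision and destroys it after a short delay.
; The spawn function places BP_Ball_Hi at the ball's location, using player pawn 0's PlayerArrow rotation with a random pitch increase.
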(event `self.Sphere.OnComponentBeginOverlap`
  (params (OverlappedComponent :type "PrimitiveComponent Object Reference") (OtherActor :type "Actor Object Reference") (OtherComp :type "PrimitiveComponent Object Reference") (OtherBodyIndex :type Integer) (bFromSweep :type Boolean) (SweepResult :type "HitResult Structure (by ref)"))
  ; Comment
  (bind _asbp_third_person_character (cast `/Game/ThirdPerson/Blueprints/BP_ThirdPersonCharacter` OtherActor))
  (bind _ascapsule_collision (cast `CapsuleComponent` OtherComp))
  (if (== _ascapsule_collision (`/Game/ThirdPerson/Blueprints/BP_ThirdPersonCharacter.Foot_Capsule` _asbp_third_person_character))
    (`/Engine/EditorBlueprintResources/StandardMacros.DoOnce` false
      (:`Completed`
        (`self.Ball_Hi_SpawnFunc`)
        ; Comment
        (`SceneComponent.SetVisibility` (`self.Ball`) false false)
        (`PrimitiveComponent.SetCollisionEnabled` (`self.Sphere`) "NoCollision")
        (`KismetSystemLibrary.Delay` 0.2)
        (`self.K2_DestroyActor`)))))

(fn `Ball_Hi_SpawnFunc`
  (bind _asbp_third_person_character (cast `/Game/ThirdPerson/Blueprints/BP_ThirdPersonCharacter` (`GameplayStatics.GetPlayerPawn` 0)))
  (bind (_returnvalue_roll _returnvalue_pitch _returnvalue_yaw) (`KismetMathLibrary.BreakRotator` (`SceneComponent.K2_GetComponentRotation` (`/Game/ThirdPerson/Blueprints/BP_ThirdPersonCharacter.Player_Arrow` _asbp_third_person_character))))
  (`|SpawnActorFromClass` "/Game/Ball/BP_Ball_Hi.BP_Ball_Hi_C" (`KismetMathLibrary.MakeTransform` (`SceneComponent.K2_GetComponentLocation` (`self.Ball`)) (`KismetMathLibrary.MakeRotator` _returnvalue_roll (+ _returnvalue_pitch (`KismetMathLibrary.RandomFloatInRange` 20.0 50.0)) _returnvalue_yaw)) "Undefined" "MultiplyWithRoot" null null))

(fn `UserConstructionScript`)