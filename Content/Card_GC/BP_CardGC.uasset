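; BP_CardGC is a destructible card actor built on a Geometry Collection that shatters as soon as it spawns.
; On BeginPlay it spawns an FS_MasterField at the collection's transform, sets its activation type and radial magnitude, triggers it, then destroys the field shortly afterwards.
; The Chaos break event starts a short delay, after which the card actor destroys itself to clean up the debris.
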(event `self.ReceiveBeginPlay`
  (bind _gc_card_gc (`self.GC_card_GC`))
  (bind _returnvalue (`|SpawnActorFromClass` "/Engine/EditorResources/FieldNodes/FS_MasterField.FS_MasterField_C" (`KismetMathLibrary.MakeTransform` (`SceneComponent.K2_GetComponentLocation` _gc_card_gc) (`SceneComponent.K2_GetComponentRotation` _gc_card_gc)) "Undefined" "MultiplyWithRoot" null null))
  (set `/Engine/EditorResources/FieldNodes/FS_MasterField.ActivationType` "NewEnumerator4" _returnvalue)
  (set `/Engine/EditorResources/FieldNodes/FS_MasterField.Radial Magnitude` 50.0 _returnvalue)
  (`/Engine/EditorResources/FieldNodes/FS_MasterField.CE_Trigger` _returnvalue)
  (`KismetSystemLibrary.Delay` 0.2)
  (`self.K2_DestroyActor` _returnvalue))

(event `self.GC_card_GC.OnChaosBreakEvent`
  (params (BreakEvent :type "ChaosBreakEvent Structure (by ref)"))
  (`KismetSystemLibrary.Delay` 5.0)
  (`self.K2_DestroyActor`))

(fn `UserConstructionScript`)