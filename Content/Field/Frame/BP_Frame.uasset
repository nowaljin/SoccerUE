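; BP_Frame is the target frame of a struck-out kicking game, holding twelve numbered cards that a Ball-tagged actor knocks out.
; Per-card box overlaps spawn BP_CardGC in place, hide the card, disable the box's collision and increment CardCounter on StruckOutGameInstnce.
; Cards 5 and 7 also adjust KickCounter, and card 6 sets GameOverFlag.
; Box 11 triggers on end overlap and Box 12 on both; CardFunc is an unused, unfinished helper.
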(event `self.Box_5.OnComponentBeginOverlap`
  (params (OverlappedComponent :type "PrimitiveComponent Object Reference") (OtherActor :type "Actor Object Reference") (OtherComp :type "PrimitiveComponent Object Reference") (OtherBodyIndex :type Integer) (bFromSweep :type Boolean) (SweepResult :type "HitResult Structure (by ref)"))
  (bind _card_5 (`self.Card_5`))
  (if (`self.ActorHasTag` OtherActor "Ball")
    (`|SpawnActorFromClass` "/Game/Field/Card/Card_GC/BP_CardGC.BP_CardGC_C" (`KismetMathLibrary.MakeTransform` (`SceneComponent.K2_GetComponentLocation` _card_5) (`SceneComponent.K2_GetComponentRotation` _card_5)) "Undefined" "MultiplyWithRoot" null null)
    (`SceneComponent.SetVisibility` (`self.Card_5`) false false)
    (`PrimitiveComponent.SetCollisionEnabled` (`self.Box_5`) "NoCollision")
    (`self.CardCounter_inc_Func`)
    ; kick -1
    (bind _asstruck_out_game_instnce (cast `/Game/StruckOutGameInstnce` (`GameplayStatics.GetGameInstance`)))
    (set `/Game/StruckOutGameInstnce.KickCounter` (- (`/Game/StruckOutGameInstnce.KickCounter` _asstruck_out_game_instnce) 1) _asstruck_out_game_instnce)))

(event `self.Box_12.OnComponentBeginOverlap`
  (params (OverlappedComponent :type "PrimitiveComponent Object Reference") (OtherActor :type "Actor Object Reference") (OtherComp :type "PrimitiveComponent Object Reference") (OtherBodyIndex :type Integer) (bFromSweep :type Boolean) (SweepResult :type "HitResult Structure (by ref)"))
  (bind _card_12 (`self.Card_12`))
  (if (`self.ActorHasTag` OtherActor "Ball")
    (`|SpawnActorFromClass` "/Game/Field/Card/Card_GC/BP_CardGC.BP_CardGC_C" (`KismetMathLibrary.MakeTransform` (`SceneComponent.K2_GetComponentLocation` _card_12) (`SceneComponent.K2_GetComponentRotation` _card_12)) "Undefined" "MultiplyWithRoot" null null)
    (`SceneComponent.SetVisibility` (`self.Card_12`) false false)
    (`PrimitiveComponent.SetCollisionEnabled` (`self.Box_12`) "NoCollision")
    (`self.CardCounter_inc_Func`)))

(event `self.Box_4.OnComponentBeginOverlap`
  (params (OverlappedComponent :type "PrimitiveComponent Object Reference") (OtherActor :type "Actor Object Reference") (OtherComp :type "PrimitiveComponent Object Reference") (OtherBodyIndex :type Integer) (bFromSweep :type Boolean) (SweepResult :type "HitResult Structure (by ref)"))
  (bind _card_4 (`self.Card_4`))
  (if (`self.ActorHasTag` OtherActor "Ball")
    (`|SpawnActorFromClass` "/Game/Field/Card/Card_GC/BP_CardGC.BP_CardGC_C" (`KismetMathLibrary.MakeTransform` (`SceneComponent.K2_GetComponentLocation` _card_4) (`SceneComponent.K2_GetComponentRotation` _card_4)) "Undefined" "MultiplyWithRoot" null null)
    (`SceneComponent.SetVisibility` (`self.Card_4`) false false)
    (`PrimitiveComponent.SetCollisionEnabled` (`self.Box_4`) "NoCollision")
    (`self.CardCounter_inc_Func`)))

(event `self.Box_6.OnComponentBeginOverlap`
  (params (OverlappedComponent :type "PrimitiveComponent Object Reference") (OtherActor :type "Actor Object Reference") (OtherComp :type "PrimitiveComponent Object Reference") (OtherBodyIndex :type Integer) (bFromSweep :type Boolean) (SweepResult :type "HitResult Structure (by ref)"))
  (bind _card_6 (`self.Card_6`))
  (if (`self.ActorHasTag` OtherActor "Ball")
    (`|SpawnActorFromClass` "/Game/Field/Card/Card_GC/BP_CardGC.BP_CardGC_C" (`KismetMathLibrary.MakeTransform` (`SceneComponent.K2_GetComponentLocation` _card_6) (`SceneComponent.K2_GetComponentRotation` _card_6)) "Undefined" "MultiplyWithRoot" null null)
    (`SceneComponent.SetVisibility` (`self.Card_6`) false false)
    (`PrimitiveComponent.SetCollisionEnabled` (`self.Box_6`) "NoCollision")
    (`self.CardCounter_inc_Func`)
    ; Game Over Flag
    (bind _asstruck_out_game_instnce (cast `/Game/StruckOutGameInstnce` (`GameplayStatics.GetGameInstance`)))
    (set `/Game/StruckOutGameInstnce.GameOverFlag` true _asstruck_out_game_instnce)))

(event `self.Box_1.OnComponentBeginOverlap`
  (params (OverlappedComponent :type "PrimitiveComponent Object Reference") (OtherActor :type "Actor Object Reference") (OtherComp :type "PrimitiveComponent Object Reference") (OtherBodyIndex :type Integer) (bFromSweep :type Boolean) (SweepResult :type "HitResult Structure (by ref)"))
  (bind _card_1 (`self.Card_1`))
  (if (`self.ActorHasTag` OtherActor "Ball")
    (`|SpawnActorFromClass` "/Game/Field/Card/Card_GC/BP_CardGC.BP_CardGC_C" (`KismetMathLibrary.MakeTransform` (`SceneComponent.K2_GetComponentLocation` _card_1) (`SceneComponent.K2_GetComponentRotation` _card_1)) "Undefined" "MultiplyWithRoot" null null)
    (`SceneComponent.SetVisibility` (`self.Card_1`) false false)
    (`PrimitiveComponent.SetCollisionEnabled` (`self.Box_1`) "NoCollision")
    (`self.CardCounter_inc_Func`)))

(event `self.Box_7.OnComponentBeginOverlap`
  (params (OverlappedComponent :type "PrimitiveComponent Object Reference") (OtherActor :type "Actor Object Reference") (OtherComp :type "PrimitiveComponent Object Reference") (OtherBodyIndex :type Integer) (bFromSweep :type Boolean) (SweepResult :type "HitResult Structure (by ref)"))
  (bind _card_7 (`self.Card_7`))
  (if (`self.ActorHasTag` OtherActor "Ball")
    (`|SpawnActorFromClass` "/Game/Field/Card/Card_GC/BP_CardGC.BP_CardGC_C" (`KismetMathLibrary.MakeTransform` (`SceneComponent.K2_GetComponentLocation` _card_7) (`SceneComponent.K2_GetComponentRotation` _card_7)) "Undefined" "MultiplyWithRoot" null null)
    (`SceneComponent.SetVisibility` (`self.Card_7`) false false)
    (`PrimitiveComponent.SetCollisionEnabled` (`self.Box_7`) "NoCollision")
    (`self.CardCounter_inc_Func`)
    ; +2 Score
    (bind _asstruck_out_game_instnce (cast `/Game/StruckOutGameInstnce` (`GameplayStatics.GetGameInstance`)))
    (set `/Game/StruckOutGameInstnce.KickCounter` (+ (`/Game/StruckOutGameInstnce.KickCounter` _asstruck_out_game_instnce) 2) _asstruck_out_game_instnce)))

(event `self.Box_2.OnComponentBeginOverlap`
  (params (OverlappedComponent :type "PrimitiveComponent Object Reference") (OtherActor :type "Actor Object Reference") (OtherComp :type "PrimitiveComponent Object Reference") (OtherBodyIndex :type Integer) (bFromSweep :type Boolean) (SweepResult :type "HitResult Structure (by ref)"))
  (bind _card_2 (`self.Card_2`))
  (if (`self.ActorHasTag` OtherActor "Ball")
    (`|SpawnActorFromClass` "/Game/Field/Card/Card_GC/BP_CardGC.BP_CardGC_C" (`KismetMathLibrary.MakeTransform` (`SceneComponent.K2_GetComponentLocation` _card_2) (`SceneComponent.K2_GetComponentRotation` _card_2)) "Undefined" "MultiplyWithRoot" null null)
    (`SceneComponent.SetVisibility` (`self.Card_2`) false false)
    (`PrimitiveComponent.SetCollisionEnabled` (`self.Box_2`) "NoCollision")
    (`self.CardCounter_inc_Func`)))

(event `self.Box_3.OnComponentBeginOverlap`
  (params (OverlappedComponent :type "PrimitiveComponent Object Reference") (OtherActor :type "Actor Object Reference") (OtherComp :type "PrimitiveComponent Object Reference") (OtherBodyIndex :type Integer) (bFromSweep :type Boolean) (SweepResult :type "HitResult Structure (by ref)"))
  (bind _card_3 (`self.Card_3`))
  (if (`self.ActorHasTag` OtherActor "Ball")
    (`|SpawnActorFromClass` "/Game/Field/Card/Card_GC/BP_CardGC.BP_CardGC_C" (`KismetMathLibrary.MakeTransform` (`SceneComponent.K2_GetComponentLocation` _card_3) (`SceneComponent.K2_GetComponentRotation` _card_3)) "Undefined" "MultiplyWithRoot" null null)
    (`SceneComponent.SetVisibility` (`self.Card_3`) false false)
    (`PrimitiveComponent.SetCollisionEnabled` (`self.Box_3`) "NoCollision")
    (`self.CardCounter_inc_Func`)))

(event `self.Box_11.OnComponentEndOverlap`
  (params (OverlappedComponent :type "PrimitiveComponent Object Reference") (OtherActor :type "Actor Object Reference") (OtherComp :type "PrimitiveComponent Object Reference") (OtherBodyIndex :type Integer))
  (bind _card_11 (`self.Card_11`))
  (if (`self.ActorHasTag` OtherActor "Ball")
    (`|SpawnActorFromClass` "/Game/Field/Card/Card_GC/BP_CardGC.BP_CardGC_C" (`KismetMathLibrary.MakeTransform` (`SceneComponent.K2_GetComponentLocation` _card_11) (`SceneComponent.K2_GetComponentRotation` _card_11)) "Undefined" "MultiplyWithRoot" null null)
    (`SceneComponent.SetVisibility` (`self.Card_11`) false false)
    (`PrimitiveComponent.SetCollisionEnabled` (`self.Box_11`) "NoCollision")
    (`self.CardCounter_inc_Func`)))

(event `self.Box_12.OnComponentEndOverlap`
  (params (OverlappedComponent :type "PrimitiveComponent Object Reference") (OtherActor :type "Actor Object Reference") (OtherComp :type "PrimitiveComponent Object Reference") (OtherBodyIndex :type Integer))
  (bind _card_12 (`self.Card_12`))
  (if (`self.ActorHasTag` OtherActor "Ball")
    (`|SpawnActorFromClass` "/Game/Field/Card/Card_GC/BP_CardGC.BP_CardGC_C" (`KismetMathLibrary.MakeTransform` (`SceneComponent.K2_GetComponentLocation` _card_12) (`SceneComponent.K2_GetComponentRotation` _card_12)) "Undefined" "MultiplyWithRoot" null null)
    (`SceneComponent.SetVisibility` (`self.Card_12`) false false)
    (`PrimitiveComponent.SetCollisionEnabled` (`self.Box_12`) "NoCollision")
    (`self.CardCounter_inc_Func`)))

(event `self.Box_8.OnComponentBeginOverlap`
  (params (OverlappedComponent :type "PrimitiveComponent Object Reference") (OtherActor :type "Actor Object Reference") (OtherComp :type "PrimitiveComponent Object Reference") (OtherBodyIndex :type Integer) (bFromSweep :type Boolean) (SweepResult :type "HitResult Structure (by ref)"))
  (bind _card_8 (`self.Card_8`))
  (if (`self.ActorHasTag` OtherActor "Ball")
    (`|SpawnActorFromClass` "/Game/Field/Card/Card_GC/BP_CardGC.BP_CardGC_C" (`KismetMathLibrary.MakeTransform` (`SceneComponent.K2_GetComponentLocation` _card_8) (`SceneComponent.K2_GetComponentRotation` _card_8)) "Undefined" "MultiplyWithRoot" null null)
    (`SceneComponent.SetVisibility` (`self.Card_8`) false false)
    (`PrimitiveComponent.SetCollisionEnabled` (`self.Box_8`) "NoCollision")
    (`self.CardCounter_inc_Func`)))

(event `self.Box_10.OnComponentBeginOverlap`
  (params (OverlappedComponent :type "PrimitiveComponent Object Reference") (OtherActor :type "Actor Object Reference") (OtherComp :type "PrimitiveComponent Object Reference") (OtherBodyIndex :type Integer) (bFromSweep :type Boolean) (SweepResult :type "HitResult Structure (by ref)"))
  (bind _card_10 (`self.Card_10`))
  (if (`self.ActorHasTag` OtherActor "Ball")
    (`|SpawnActorFromClass` "/Game/Field/Card/Card_GC/BP_CardGC.BP_CardGC_C" (`KismetMathLibrary.MakeTransform` (`SceneComponent.K2_GetComponentLocation` _card_10) (`SceneComponent.K2_GetComponentRotation` _card_10)) "Undefined" "MultiplyWithRoot" null null)
    (`SceneComponent.SetVisibility` (`self.Card_10`) false false)
    (`PrimitiveComponent.SetCollisionEnabled` (`self.Box_10`) "NoCollision")
    (`self.CardCounter_inc_Func`)))

(event `self.Box_9.OnComponentBeginOverlap`
  (params (OverlappedComponent :type "PrimitiveComponent Object Reference") (OtherActor :type "Actor Object Reference") (OtherComp :type "PrimitiveComponent Object Reference") (OtherBodyIndex :type Integer) (bFromSweep :type Boolean) (SweepResult :type "HitResult Structure (by ref)"))
  (bind _card_9 (`self.Card_9`))
  (if (`self.ActorHasTag` OtherActor "Ball")
    (`|SpawnActorFromClass` "/Game/Field/Card/Card_GC/BP_CardGC.BP_CardGC_C" (`KismetMathLibrary.MakeTransform` (`SceneComponent.K2_GetComponentLocation` _card_9) (`SceneComponent.K2_GetComponentRotation` _card_9)) "Undefined" "MultiplyWithRoot" null null)
    (`SceneComponent.SetVisibility` (`self.Card_9`) false false)
    (`PrimitiveComponent.SetCollisionEnabled` (`self.Box_9`) "NoCollision")
    (`self.CardCounter_inc_Func`)))

(fn `CardCounter_inc_Func`
  (bind _asstruck_out_game_instnce (cast `/Game/StruckOutGameInstnce` (`GameplayStatics.GetGameInstance`)))
  (`/Engine/EditorBlueprintResources/StandardMacros.IncrementInt` (`/Game/StruckOutGameInstnce.CardCounter` _asstruck_out_game_instnce)))

(fn `CardFunc`
  (params (Box :type "SceneComponent Object Reference") (Mesh :type "SceneComponent Object Reference"))
  (`|SpawnActorFromClass` "/Game/Field/Card/Card_GC/BP_CardGC.BP_CardGC_C" (`KismetMathLibrary.MakeTransform` (`SceneComponent.K2_GetComponentLocation` Box) (`SceneComponent.K2_GetComponentRotation` Mesh)) "Undefined" "MultiplyWithRoot" null null))

(fn `UserConstructionScript`)