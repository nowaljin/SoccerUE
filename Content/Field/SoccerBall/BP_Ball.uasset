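; BP_Ball is the stationary soccer ball in what appears to be a Struck Out kicking game, waiting to be kicked by BP_Soccer.
; A one-shot overlap with the player's foot capsule increments the game instance's kick counter and picks Mid, Hi or Low from KickST.
; It spawns that ball class along the player's arrow with random added pitch (plus a yaw offset for Low), then hides itself and self-destroys after a delay.
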(event `self.Sphere.OnComponentBeginOverlap`
  (params (OverlappedComponent :type "PrimitiveComponent Object Reference") (OtherActor :type "Actor Object Reference") (OtherComp :type "PrimitiveComponent Object Reference") (OtherBodyIndex :type Integer) (bFromSweep :type Boolean) (SweepResult :type "HitResult Structure (by ref)"))
  (bind _asbp_soccer (cast `/Game/Player/BP_Soccer` OtherActor))
  ; Playerの右足のカプセルと当たったか
  (bind _ascapsule_collision (cast `CapsuleComponent` OtherComp))
  (if (== _ascapsule_collision (`/Game/Player/BP_Soccer.Foot_Capsule` _asbp_soccer))
    (`/Engine/EditorBlueprintResources/StandardMacros.DoOnce` false
      (:`Completed`
        (bind _asstruck_out_game_instnce (cast `/Game/StruckOutGameInstnce` (`GameplayStatics.GetGameInstance`)))
        ; ボールを動かす
        (`/Engine/EditorBlueprintResources/StandardMacros.IncrementInt` (`/Game/StruckOutGameInstnce.KickCounter` _asstruck_out_game_instnce)
          (:`  `
            (switch `int` (`/Game/Player/BP_Soccer.Kick_ST` _asbp_soccer)
              (:`0`
                (`self.Ball_Mid_SpawnFunc`))
              (:`1`
                (`self.Ball_Hi_SpawnFunc`))
              (:`2`
                (`self.Ball_Low_SpawnFunc`)))
            ; 次のボールを出現させる時間
            (`SceneComponent.SetVisibility` (`self.SoccerBall`) false false)
            (`PrimitiveComponent.SetCollisionEnabled` (`self.Sphere`) "NoCollision")
            (`KismetSystemLibrary.Delay` 4.0)
            (`self.K2_DestroyActor`)))))))

(fn `Ball_Hi_SpawnFunc`
  (bind _asbp_soccer (cast `/Game/Player/BP_Soccer` (`GameplayStatics.GetPlayerPawn` 0)))
  (bind (_returnvalue_roll _returnvalue_pitch _returnvalue_yaw) (`KismetMathLibrary.BreakRotator` (`SceneComponent.K2_GetComponentRotation` (`/Game/Player/BP_Soccer.PlayerArrow` _asbp_soccer))))
  (`|SpawnActorFromClass` "/Game/Field/SoccerBall/BP_Ball_Hi.BP_Ball_Hi_C" (`KismetMathLibrary.MakeTransform` (`SceneComponent.K2_GetComponentLocation` (`self.SoccerBall`)) (`KismetMathLibrary.MakeRotator` _returnvalue_roll (+ _returnvalue_pitch (`KismetMathLibrary.RandomFloatInRange` 18.0 23.0)) _returnvalue_yaw)) "Undefined" "MultiplyWithRoot" null null))

(fn `Ball_Low_SpawnFunc`
  (bind _asbp_soccer (cast `/Game/Player/BP_Soccer` (`GameplayStatics.GetPlayerPawn` 0)))
  (bind (_returnvalue_roll _returnvalue_pitch _returnvalue_yaw) (`KismetMathLibrary.BreakRotator` (`SceneComponent.K2_GetComponentRotation` (`/Game/Player/BP_Soccer.PlayerArrow` _asbp_soccer))))
  (`|SpawnActorFromClass` "/Game/Field/SoccerBall/BP_Ball_Low.BP_Ball_Low_C" (`KismetMathLibrary.MakeTransform` (`SceneComponent.K2_GetComponentLocation` (`self.SoccerBall`)) (`KismetMathLibrary.MakeRotator` _returnvalue_roll (+ _returnvalue_pitch (`KismetMathLibrary.RandomFloatInRange` 10.0 15.0)) (+ _returnvalue_yaw 20.0))) "Undefined" "MultiplyWithRoot" null null))

(fn `Ball_Mid_SpawnFunc`
  (bind _asbp_soccer (cast `/Game/Player/BP_Soccer` (`GameplayStatics.GetPlayerPawn` 0)))
  (bind (_returnvalue_roll _returnvalue_pitch _returnvalue_yaw) (`KismetMathLibrary.BreakRotator` (`SceneComponent.K2_GetComponentRotation` (`/Game/Player/BP_Soccer.PlayerArrow` _asbp_soccer))))
  (`|SpawnActorFromClass` "/Game/Field/SoccerBall/BP_Ball_Mid.BP_Ball_Mid_C" (`KismetMathLibrary.MakeTransform` (`SceneComponent.K2_GetComponentLocation` (`self.SoccerBall`)) (`KismetMathLibrary.MakeRotator` _returnvalue_roll (+ _returnvalue_pitch (`KismetMathLibrary.RandomFloatInRange` 15.0 19.0)) _returnvalue_yaw)) "Undefined" "MultiplyWithRoot" null null))

(fn `UserConstructionScript`)