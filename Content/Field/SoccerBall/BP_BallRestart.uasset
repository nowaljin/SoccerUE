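; BP_BallRestart keeps a soccer ball in play on the field by respawning BP_Ball whenever none exists in the level.
; Every Tick it gathers all BP_Ball actors, and if the list is empty it spawns a new one.
; The spawn location is a random point inside its Box component, and the rotation comes from its Arrow component.
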(event `self.ReceiveTick`
  (params (DeltaSeconds :type "Float (single-precision)"))
  (bind _box (`self.Box`))
  (bind _outactors (`GameplayStatics.GetAllActorsOfClass` "/Game/Field/SoccerBall/BP_Ball.BP_Ball_C"))
  (if (< (`KismetArrayLibrary.Array_Length` _outactors) 1)
    (`|SpawnActorFromClass` "/Game/Field/SoccerBall/BP_Ball.BP_Ball_C" (`KismetMathLibrary.MakeTransform` (`KismetMathLibrary.RandomPointInBoundingBox` (`SceneComponent.K2_GetComponentLocation` _box) (`BoxComponent.BoxExtent` _box)) (`SceneComponent.K2_GetComponentRotation` (`self.Arrow`))) "Undefined" "MultiplyWithRoot" null null)))

(fn `UserConstructionScript`)