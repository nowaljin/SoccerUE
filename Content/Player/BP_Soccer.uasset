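; BP_Soccer is the player-controlled soccer character, with movement, look, jump and three kick actions.
; On possession it adds the IMC_Player Enhanced Input mapping context, then moves relative to control yaw.
; Left mouse, right mouse and Q play separate kick montages on the mesh.
; CollisionON and CollisionOFF events toggle the foot capsule's collision, with no caller in this graph.
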(event `self.ReceivePossessed`
  (params (NewController :type "Controller Object Reference"))
  (bind _asplayer_controller (cast `PlayerController` NewController))
  (message `EnhancedInputSubsystemInterface.AddMappingContext` (pcsubsystem `EnhancedInputLocalPlayerSubsystem` _asplayer_controller) "/Game/Input/IMC_Player.IMC_Player" 0 (struct)))

(event `EnhancedInput|/Game/Input/IA_MouseL`
  (params (ActionValue :type Boolean) (ElapsedSeconds :type "Float (double-precision)") (TriggeredSeconds :type "Float (double-precision)") (InputAction :type "InputAction Object Reference" :default "/Game/Input/IA_MouseL.IA_MouseL"))
  (:`Triggered`
    (`|PlayMontage` (`self.Mesh`) "/Game/Player/Animation/KickBallMTG.KickBallMTG")))

(event `EnhancedInput|/Game/Input/IA_Jump`
  (params (ActionValue :type Boolean) (ElapsedSeconds :type "Float (double-precision)") (TriggeredSeconds :type "Float (double-precision)") (InputAction :type "InputAction Object Reference" :default "/Game/Input/IA_Jump.IA_Jump"))
  (:`Triggered`
    (`self.Jump`)))

(event `EnhancedInput|/Game/Input/IA_Turn`
  (params (ActionValue :type "Float (double-precision)") (ElapsedSeconds :type "Float (double-precision)") (TriggeredSeconds :type "Float (double-precision)") (InputAction :type "InputAction Object Reference" :default "/Game/Input/IA_Turn.IA_Turn"))
  (:`Triggered`
    (`self.AddControllerYawInput` ActionValue)))

(event `EnhancedInput|/Game/Input/IA_MouseR`
  (params (ActionValue :type Boolean) (ElapsedSeconds :type "Float (double-precision)") (TriggeredSeconds :type "Float (double-precision)") (InputAction :type "InputAction Object Reference" :default "/Game/Input/IA_MouseR.IA_MouseR"))
  (:`Triggered`
    (`|PlayMontage` (`self.Mesh`) "/Game/Player/Animation/Kick_LongMTG.Kick_LongMTG")))

(event `EnhancedInput|/Game/Input/IA_LookUp`
  (params (ActionValue :type "Float (double-precision)") (ElapsedSeconds :type "Float (double-precision)") (TriggeredSeconds :type "Float (double-precision)") (InputAction :type "InputAction Object Reference" :default "/Game/Input/IA_LookUp.IA_LookUp"))
  (:`Triggered`
    (`self.AddControllerPitchInput` ActionValue)))

(event `EnhancedInput|/Game/Input/IA_Q`
  (params (ActionValue :type Boolean) (ElapsedSeconds :type "Float (double-precision)") (TriggeredSeconds :type "Float (double-precision)") (InputAction :type "InputAction Object Reference" :default "/Game/Input/IA_Q.IA_Q"))
  (:`Triggered`
    (`|PlayMontage` (`self.Mesh`) "/Game/Player/Animation/KickBallshortMTG.KickBallshortMTG")))

(event `EnhancedInput|/Game/Input/IA_WS`
  (params (ActionValue :type "Float (double-precision)") (ElapsedSeconds :type "Float (double-precision)") (TriggeredSeconds :type "Float (double-precision)") (InputAction :type "InputAction Object Reference" :default "/Game/Input/IA_WS.IA_WS"))
  (bind (_returnvalue_roll _returnvalue_pitch _returnvalue_yaw) (`KismetMathLibrary.BreakRotator` (`self.GetControlRotation`)))
  (:`Triggered`
    (`self.AddMovementInput` (`KismetMathLibrary.GetForwardVector` (`KismetMathLibrary.MakeRotator` 0.0 0.0 _returnvalue_yaw)) (* ActionValue 1.0))))

(event `CollisionON`
  ; 足の当たり判定 ON/OFF
  (`PrimitiveComponent.SetCollisionEnabled` (`self.Foot_Capsule`) "QueryAndPhysics"))

(event `EnhancedInput|/Game/Input/IA_AD`
  (params (ActionValue :type "Float (double-precision)") (ElapsedSeconds :type "Float (double-precision)") (TriggeredSeconds :type "Float (double-precision)") (InputAction :type "InputAction Object Reference" :default "/Game/Input/IA_AD.IA_AD"))
  (bind (_returnvalue_roll _returnvalue_pitch _returnvalue_yaw) (`KismetMathLibrary.BreakRotator` (`self.GetControlRotation`)))
  (:`Triggered`
    (`self.AddMovementInput` (`KismetMathLibrary.GetRightVector` (`KismetMathLibrary.MakeRotator` 0.0 0.0 _returnvalue_yaw)) (* ActionValue 1.0))))

(event `CollisionOFF`
  ; 足の当たり判定 ON/OFF
  (`PrimitiveComponent.SetCollisionEnabled` (`self.Foot_Capsule`) "NoCollision"))

(fn `UserConstructionScript`)